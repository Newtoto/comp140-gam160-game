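; Player controller for a four-turret game that takes aim and fire input from the keyboard or an Arduino, and menu input from the Arduino.
; Keys 1–4 possess and tint a turret, while Tick rotates it or applies length-checked Arduino serial values to a turret pair.
; Arduino "F" switches pairs, then starts projectiles.
; In level select or once all turrets finish firing, Arduino readings become menu X/Y and selection.
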(event EventBeginPlay
  (bind _returnvalue (Game|GetCurrentLevelName true))
  (bind _output_get (Variables|Default|SetIsLevelSelect (Utilities|Enum|Equal(Enum) _returnvalue "LevelSelect")))
  (if (not _output_get)
    ;[1 1 1] Auto select first turret on begin play
    (bind _outactors (Actor|GetAllActorsOfClass "/Game/2DSideScrollerBP/Blueprints/TurretPawnBP.TurretPawnBP_C"))
    (bind _output_get_2 (Variables|Default|SetAvailableTurrets _outactors))
    (Pawn|Possess (Utilities|Array|Get(acopy) _output_get_2 (Variables|Default|GetSelectedTurretIndex)))
    (if (Variables|Default|GetUsingArduino)
      (Sprite|SetSpriteColor (Variables|/Game/2DSideScrollerBP/Blueprints/TurretPawnBP.TurretPawnBP_C|GetTurret (Utilities|Array|Get(acopy) _output_get_2 1)) "(R=0.550000,G=0.550000,B=0.550000,A=1.000000)"))
    (Sprite|SetSpriteColor (Variables|/Game/2DSideScrollerBP/Blueprints/TurretPawnBP.TurretPawnBP_C|GetTurret (Utilities|Array|Get(acopy) _output_get_2 (Variables|Default|GetSelectedTurretIndex))) "(R=0.550000,G=0.550000,B=0.550000,A=1.000000)")))

(event EventTick
  (params (DeltaSeconds :type Float%20%28single-precision%29))
  (if (Variables|Default|GetTurretsFinishedFiring)
    (CallFunction|ParseArduinoforMenu :!label _label)
    (elif (Variables|Default|GetIsLevelSelect)
      (goto _label)
      (elif (Variables|Default|GetStartProjectiles)
        (if (not (Variables|Default|GetTurretsFinishedFiring))
          (bind _array_element (Utilities|Array|ForEachLoopwithBreak (Variables|Default|GetAvailableTurrets))
            (:LoopBody
              (if (== (Variables|/Game/2DSideScrollerBP/Blueprints/TurretPawnBP.TurretPawnBP_C|GetShotsFired _array_element) (Variables|/Game/2DSideScrollerBP/Blueprints/TurretPawnBP.TurretPawnBP_C|GetNumberOfShots _array_element))
                (bind _result (Math|Integer|IncrementInt (Variables|Default|GetFinishedTurrets))
                  (:%20%20
                    (Variables|Default|SetFinishedTurrets _result)))))
            (:Completed
              (if (== (Variables|Default|GetFinishedTurrets) 4)
                (Variables|Default|SetTurretsFinishedFiring true)
                (else
                  (Variables|Default|SetFinishedTurrets 0))))))
        (elif (Variables|Default|GetUsingArduino)
          (CallFunction|ParseArduinoStringforRotation)
          (else
            ;[1 1 1] Set rotation from keyboard input
            (Transformation|AddWorldRotation (Variables|/Game/2DSideScrollerBP/Blueprints/TurretPawnBP.TurretPawnBP_C|GetTurret (Utilities|Array|Get(acopy) (Variables|Default|GetAvailableTurrets) (Variables|Default|GetSelectedTurretIndex))) (Variables|Default|GetTurretRotation) false false)))))))

(event Input|KeyboardEvents|1
  (params (Key :type Key%20Structure :default "AnyKey"))
  ;[1 1 1] Keyboard Turret Switching
  (:Pressed
    (Variables|Default|SetPreviousTurretIndex (Variables|Default|GetSelectedTurretIndex))
    (Variables|Default|SetSelectedTurretIndex 0)
    (if (not (Variables|Default|GetIsLevelSelect))
      (Utilities|Casting|CastToTurretPawnBPClass "/Game/2DSideScrollerBP/Blueprints/TurretPawnBP.TurretPawnBP_C")
      ;;[1 1 1] Reset previous turret and activate new turret
      (Variables|/Game/2DSideScrollerBP/Blueprints/TurretPawnBP.TurretPawnBP_C|SetRotateLeft (Utilities|Array|Get(acopy) (Variables|Default|GetAvailableTurrets) (Variables|Default|GetPreviousTurretIndex)) false)
      (Variables|/Game/2DSideScrollerBP/Blueprints/TurretPawnBP.TurretPawnBP_C|SetRotateRight (Utilities|Array|Get(acopy) (Variables|Default|GetAvailableTurrets) (Variables|Default|GetPreviousTurretIndex)) false)
      (Sprite|SetSpriteColor (Variables|/Game/2DSideScrollerBP/Blueprints/TurretPawnBP.TurretPawnBP_C|GetTurret (Utilities|Array|Get(acopy) (Variables|Default|GetAvailableTurrets) (Variables|Default|GetPreviousTurretIndex))) "(R=1.000000,G=1.000000,B=1.000000,A=1.000000)")
      (Pawn|Possess (Utilities|Array|Get(acopy) (Variables|Default|GetAvailableTurrets) (Variables|Default|GetSelectedTurretIndex)))
      (Sprite|SetSpriteColor (Variables|/Game/2DSideScrollerBP/Blueprints/TurretPawnBP.TurretPawnBP_C|GetTurret (Utilities|Array|Get(acopy) (Variables|Default|GetAvailableTurrets) (Variables|Default|GetSelectedTurretIndex))) "(R=0.550000,G=0.550000,B=0.550000,A=1.000000)"))))

(event Input|KeyboardEvents|2
  (params (Key :type Key%20Structure :default "AnyKey"))
  ;[1 1 1] Keyboard Turret Switching
  (:Pressed
    (Variables|Default|SetPreviousTurretIndex (Variables|Default|GetSelectedTurretIndex))
    (Variables|Default|SetSelectedTurretIndex 1)
    (if (not (Variables|Default|GetIsLevelSelect))
      (Utilities|Casting|CastToTurretPawnBPClass "/Game/2DSideScrollerBP/Blueprints/TurretPawnBP.TurretPawnBP_C")
      ;;[1 1 1] Reset previous turret and activate new turret
      (Variables|/Game/2DSideScrollerBP/Blueprints/TurretPawnBP.TurretPawnBP_C|SetRotateLeft (Utilities|Array|Get(acopy) (Variables|Default|GetAvailableTurrets) (Variables|Default|GetPreviousTurretIndex)) false)
      (Variables|/Game/2DSideScrollerBP/Blueprints/TurretPawnBP.TurretPawnBP_C|SetRotateRight (Utilities|Array|Get(acopy) (Variables|Default|GetAvailableTurrets) (Variables|Default|GetPreviousTurretIndex)) false)
      (Sprite|SetSpriteColor (Variables|/Game/2DSideScrollerBP/Blueprints/TurretPawnBP.TurretPawnBP_C|GetTurret (Utilities|Array|Get(acopy) (Variables|Default|GetAvailableTurrets) (Variables|Default|GetPreviousTurretIndex))) "(R=1.000000,G=1.000000,B=1.000000,A=1.000000)")
      (Pawn|Possess (Utilities|Array|Get(acopy) (Variables|Default|GetAvailableTurrets) (Variables|Default|GetSelectedTurretIndex)))
      (Sprite|SetSpriteColor (Variables|/Game/2DSideScrollerBP/Blueprints/TurretPawnBP.TurretPawnBP_C|GetTurret (Utilities|Array|Get(acopy) (Variables|Default|GetAvailableTurrets) (Variables|Default|GetSelectedTurretIndex))) "(R=0.550000,G=0.550000,B=0.550000,A=1.000000)"))))

(event Input|KeyboardEvents|3
  (params (Key :type Key%20Structure :default "AnyKey"))
  ;[1 1 1] Keyboard Turret Switching
  (:Pressed
    (Variables|Default|SetPreviousTurretIndex (Variables|Default|GetSelectedTurretIndex))
    (Variables|Default|SetSelectedTurretIndex 2)
    (if (not (Variables|Default|GetIsLevelSelect))
      (Utilities|Casting|CastToTurretPawnBPClass "/Game/2DSideScrollerBP/Blueprints/TurretPawnBP.TurretPawnBP_C")
      ;;[1 1 1] Reset previous turret and activate new turret
      (Variables|/Game/2DSideScrollerBP/Blueprints/TurretPawnBP.TurretPawnBP_C|SetRotateLeft (Utilities|Array|Get(acopy) (Variables|Default|GetAvailableTurrets) (Variables|Default|GetPreviousTurretIndex)) false)
      (Variables|/Game/2DSideScrollerBP/Blueprints/TurretPawnBP.TurretPawnBP_C|SetRotateRight (Utilities|Array|Get(acopy) (Variables|Default|GetAvailableTurrets) (Variables|Default|GetPreviousTurretIndex)) false)
      (Sprite|SetSpriteColor (Variables|/Game/2DSideScrollerBP/Blueprints/TurretPawnBP.TurretPawnBP_C|GetTurret (Utilities|Array|Get(acopy) (Variables|Default|GetAvailableTurrets) (Variables|Default|GetPreviousTurretIndex))) "(R=1.000000,G=1.000000,B=1.000000,A=1.000000)")
      (Pawn|Possess (Utilities|Array|Get(acopy) (Variables|Default|GetAvailableTurrets) (Variables|Default|GetSelectedTurretIndex)))
      (Sprite|SetSpriteColor (Variables|/Game/2DSideScrollerBP/Blueprints/TurretPawnBP.TurretPawnBP_C|GetTurret (Utilities|Array|Get(acopy) (Variables|Default|GetAvailableTurrets) (Variables|Default|GetSelectedTurretIndex))) "(R=0.550000,G=0.550000,B=0.550000,A=1.000000)"))))

(event Input|KeyboardEvents|4
  (params (Key :type Key%20Structure :default "AnyKey"))
  ;[1 1 1] Keyboard Turret Switching
  (:Pressed
    (Variables|Default|SetPreviousTurretIndex (Variables|Default|GetSelectedTurretIndex))
    (Variables|Default|SetSelectedTurretIndex 3)
    (if (not (Variables|Default|GetIsLevelSelect))
      (Utilities|Casting|CastToTurretPawnBPClass "/Game/2DSideScrollerBP/Blueprints/TurretPawnBP.TurretPawnBP_C")
      ;;[1 1 1] Reset previous turret and activate new turret
      (Variables|/Game/2DSideScrollerBP/Blueprints/TurretPawnBP.TurretPawnBP_C|SetRotateLeft (Utilities|Array|Get(acopy) (Variables|Default|GetAvailableTurrets) (Variables|Default|GetPreviousTurretIndex)) false)
      (Variables|/Game/2DSideScrollerBP/Blueprints/TurretPawnBP.TurretPawnBP_C|SetRotateRight (Utilities|Array|Get(acopy) (Variables|Default|GetAvailableTurrets) (Variables|Default|GetPreviousTurretIndex)) false)
      (Sprite|SetSpriteColor (Variables|/Game/2DSideScrollerBP/Blueprints/TurretPawnBP.TurretPawnBP_C|GetTurret (Utilities|Array|Get(acopy) (Variables|Default|GetAvailableTurrets) (Variables|Default|GetPreviousTurretIndex))) "(R=1.000000,G=1.000000,B=1.000000,A=1.000000)")
      (Pawn|Possess (Utilities|Array|Get(acopy) (Variables|Default|GetAvailableTurrets) (Variables|Default|GetSelectedTurretIndex)))
      (Sprite|SetSpriteColor (Variables|/Game/2DSideScrollerBP/Blueprints/TurretPawnBP.TurretPawnBP_C|GetTurret (Utilities|Array|Get(acopy) (Variables|Default|GetAvailableTurrets) (Variables|Default|GetSelectedTurretIndex))) "(R=0.550000,G=0.550000,B=0.550000,A=1.000000)"))))

(fn ConstructionScript)

(fn ParseArduinoStringforRotation
  (if (Utilities|String|Contains (Variables|Default|GetArduinoInput) "F")
    ;[1 1 1] Switch turrets and fire on button press
    (if (Variables|Default|GetSwitchedTurrets)
      (Variables|Default|SetStartProjectiles true)
      (else
        (Variables|Default|SetSwitchedTurrets true)
        (for _index (range 0 1)
          (Sprite|SetSpriteColor (Variables|/Game/2DSideScrollerBP/Blueprints/TurretPawnBP.TurretPawnBP_C|GetTurret (Utilities|Array|Get(acopy) (Variables|Default|GetAvailableTurrets) _index)) "(R=1.000000,G=1.000000,B=1.000000,A=1.000000)"))
        (for _index_2 (range 2 3)
          (Sprite|SetSpriteColor (Variables|/Game/2DSideScrollerBP/Blueprints/TurretPawnBP.TurretPawnBP_C|GetTurret (Utilities|Array|Get(acopy) (Variables|Default|GetAvailableTurrets) _index_2)) "(R=0.549020,G=0.549020,B=0.549020,A=1.000000)"))))
    (else
      (for _array_element (Utilities|String|ParseIntoArray (Variables|Default|GetArduinoInput) ",")
        (if (== (Math|Integer|%(Integer) (Math|Conversions|ToInteger(Byte) (Utilities|Array|Get(acopy) (Utilities|String|ParseIntoArray _array_element ":") 2)) 2) 0)
          (Variables|Default|SetTurretValue (Math|Conversions|ToInteger(Byte) (Utilities|Array|Get(acopy) (Utilities|String|ParseIntoArray _array_element ":") 2)))
          (else
            (Variables|Default|SetTurretValue (+ (Math|Conversions|ToInteger(Byte) (Utilities|Array|Get(acopy) (Utilities|String|ParseIntoArray _array_element ":") 2)) 1))))
        (if (and (== (Math|Conversions|ToInteger(Byte) (Utilities|Array|Get(acopy) (Utilities|String|ParseIntoArray _array_element ":") 1)) (Utilities|String|Len (Utilities|Array|Get(acopy) (Utilities|String|ParseIntoArray _array_element ":") 2))) (> (Math|Conversions|ToInteger(Byte) (Utilities|Array|Get(acopy) (Utilities|String|ParseIntoArray _array_element ":") 1)) 0))
          (if (Variables|Default|GetSwitchedTurrets)
            (Transformation|SetWorldRotation (Variables|/Game/2DSideScrollerBP/Blueprints/TurretPawnBP.TurretPawnBP_C|GetTurret (Utilities|Array|Get(acopy) (Variables|Default|GetAvailableTurrets) (+ (Math|Conversions|ToInteger(Byte) (Utilities|Array|Get(acopy) (Utilities|String|ParseIntoArray _array_element ":"))) 2))) (Math|Rotator|MakeRotator 0.0 (Math|Conversions|ToFloat(Integer) (Variables|Default|GetTurretValue)) 0.0) false false)
            (else
              (Transformation|SetWorldRotation (Variables|/Game/2DSideScrollerBP/Blueprints/TurretPawnBP.TurretPawnBP_C|GetTurret (Utilities|Array|Get(acopy) (Variables|Default|GetAvailableTurrets) (Math|Conversions|ToInteger(Byte) (Utilities|Array|Get(acopy) (Utilities|String|ParseIntoArray _array_element ":"))))) (Math|Rotator|MakeRotator 0.0 (Math|Conversions|ToFloat(Integer) (Variables|Default|GetTurretValue)) 0.0) false false))))))))

(fn ParseArduinoforMenu
  (if (Utilities|String|Contains (Variables|Default|GetArduinoInput) "F")
    (Variables|Default|SetArduinoSelected true)
    (else
      (for _array_element (Utilities|String|ParseIntoArray (Variables|Default|GetArduinoInput) ",")
        (Variables|Default|SetTurretValue (Math|Conversions|ToInteger(Byte) (Utilities|Array|Get(acopy) (Utilities|String|ParseIntoArray _array_element ":") 2)))
        (if (and (== (Math|Conversions|ToInteger(Byte) (Utilities|Array|Get(acopy) (Utilities|String|ParseIntoArray _array_element ":") 1)) (Utilities|String|Len (Utilities|Array|Get(acopy) (Utilities|String|ParseIntoArray _array_element ":") 2))) (> (Math|Conversions|ToInteger(Byte) (Utilities|Array|Get(acopy) (Utilities|String|ParseIntoArray _array_element ":") 1)) 0))
          (switch int (/ (+ (Variables|Default|GetTurretValue) 84) 56)
            (:0
              (bind _output_get (Variables|Default|SetTurretValue 3)))
            (:1
              (Variables|Default|SetTurretValue 2))
            (:2
              (Variables|Default|SetTurretValue 1))
            (:3
              (Variables|Default|SetTurretValue 0)))
          (switch int (Math|Conversions|ToInteger(Byte) (Utilities|Array|Get(acopy) (Utilities|String|ParseIntoArray _array_element ":")))
            (:0
              (Variables|Default|SetArduinoY _output_get))
            (:1
              (Variables|Default|SetArduinoX _output_get))))))))